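; Spawn point that creates mall agents at its own transform while the player pawn's population is below its maximum.
; Tick accumulates a cooldown, then spawns a MallAgentCPP, attaches it to the spawn point and resets the timer.
; Each spawn increments the point's own population count, which ScorePopulation normalises and maps through a curve into a utility value.
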(event `self.ReceiveTick`
  (params (DeltaSeconds :type "Float (single-precision)"))
  ;[1 1 1] If the max population has not been reached/exceeded...
  (bind _asmall_player_pawn (cast `MallPlayerPawn` (`GameplayStatics.GetPlayerPawn` 0)))
  (bind _returnvalue (`MallPlayerPawn.GetMaxPopulation` _asmall_player_pawn))
  (bind _returnvalue_2 (`MallPlayerPawn.GetPopulation` _asmall_player_pawn))
  (if (< _returnvalue_2 _returnvalue)
    ;[1 1 1] If the spawn cooldown has finished...
    (bind _output_get (set `self.currentCooldown` (+ DeltaSeconds (`self.currentCooldown`))))
    (if (>= _output_get (`self.spawnCooldown`))
      ;[1 1 1] Spawn a new mall agent, and increment the population total.
      (bind _returnvalue_3 (`|SpawnActorFromClass` "/Game/Blueprints/Agent/MallAgentCPP.MallAgentCPP_C" (`self.GetTransform`) "AdjustIfPossibleButAlwaysSpawn" "OverrideRootScale" self null))
      (`self.K2_AttachToActor` _returnvalue_3 self "None" "KeepWorld" "KeepWorld" "KeepWorld" false)
      (set `self.currentCooldown` 0.0)
      (`/Engine/EditorBlueprintResources/StandardMacros.IncrementInt` (`self.currentPopulation`)
        (:`  `
          (`self.ScorePopulation`))))))

(fn `ScorePopulation`
  (set `self.populationUtility` (`CurveFloat.GetFloatValue` (`self.PopulationCurve`) (/ (`KismetMathLibrary.Conv_IntToDouble` (`self.currentPopulation`)) (`KismetMathLibrary.Conv_IntToDouble` (`self.maxPopulation`))))))

(fn `UserConstructionScript`)