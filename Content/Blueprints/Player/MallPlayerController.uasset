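; Player controller for a mall game that drives the camera pawn and handles mouse selection.
; Input moves the pawn and zooms its spring arm within limits, with pan speed scaling with arm length.
; Tick traces under the cursor for agents, interactables and placement zones.
; Left click selects the hovered actor and opens the matching debug tool or building menu, while right click clears selection and widgets.
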(event `self.ReceiveBeginPlay`
  (`self.GetCameraRef`))

(event `InputAction|ZoomIn`
  (params (Key :type "Key Structure"))
  ;[1 1 1] Camera Zoom
  (:`Pressed`
    (set `SpringArmComponent.TargetArmLength` (`KismetMathLibrary.FClamp` (- (`SpringArmComponent.TargetArmLength` (`/Game/Blueprints/Player/MallPlayerPawn.SpringArm` (`self.CameraPawn`))) (`self.ZoomRate`)) (`self.MinZoomDistance`) (`self.MaxZoomDistance`)) (`/Game/Blueprints/Player/MallPlayerPawn.SpringArm` (`self.CameraPawn`)))))

(event `InputAction|ZoomOut`
  (params (Key :type "Key Structure"))
  ;[1 1 1] Camera Zoom
  (:`Pressed`
    (set `SpringArmComponent.TargetArmLength` (`KismetMathLibrary.FClamp` (+ (`SpringArmComponent.TargetArmLength` (`/Game/Blueprints/Player/MallPlayerPawn.SpringArm` (`self.CameraPawn`))) (`self.ZoomRate`)) (`self.MinZoomDistance`) (`self.MaxZoomDistance`)) (`/Game/Blueprints/Player/MallPlayerPawn.SpringArm` (`self.CameraPawn`)))))

(event `InputAxis|MoveForward`
  (params (AxisValue :type "Float (single-precision)"))
  ;[1 1 1] Move Camera Forward/Backwards
  (`self.K2_SetActorTransform` (`self.CameraPawn`) (`self.MoveX` (`self.MoveSpeedCalc`) (`self.MoveSensitivity`) AxisValue (`self.CameraPawn`)) false false))

(event `InputAxis|MoveRight`
  (params (AxisValue :type "Float (single-precision)"))
  ;[1 1 1] Move Camera Left/Right
  (`self.K2_SetActorTransform` (`self.CameraPawn`) (`KismetMathLibrary.MakeTransform` (`KismetMathLibrary.MakeVector` (.x (.location (`self.MoveY` (`self.MoveSpeedCalc`) (`self.MoveSensitivity`) AxisValue (`self.CameraPawn`)))) (.y (.location (`self.MoveY` (`self.MoveSpeedCalc`) (`self.MoveSensitivity`) AxisValue (`self.CameraPawn`)))) (`self.InitialCameraHeight`)) (.rotation (`self.MoveY` (`self.MoveSpeedCalc`) (`self.MoveSensitivity`) AxisValue (`self.CameraPawn`))) (.scale (`self.MoveY` (`self.MoveSpeedCalc`) (`self.MoveSensitivity`) AxisValue (`self.CameraPawn`)))) false false))

(event `InputAction|ResetZoom`
  (params (Key :type "Key Structure"))
  ;[1 1 1] Reset Camera Zoom
  (:`Pressed`
    (set `SpringArmComponent.TargetArmLength` (/ (`self.MaxZoomDistance`) 2.0) (`/Game/Blueprints/Player/MallPlayerPawn.SpringArm` (`self.CameraPawn`)))))

(event `Key|RightMouseButton`
  (params (Key :type "Key Structure"))
  ;[1 1 1] Deselect Everything
  (:`Pressed`
    (set `self.HitActor` null)
    (`WidgetLayoutLibrary.RemoveAllWidgets`)))

(event `self.ReceiveTick`
  (params (DeltaSeconds :type "Float (single-precision)"))
  (bind (_bblockinghit _binitialoverlap _time _distance _location _impactpoint _normal _impactnormal _physmat _hitactor) (`GameplayStatics.BreakHitResult` (`self.GetHitResultUnderCursorByChannel` (`GameplayStatics.GetPlayerController` 0) "TraceTypeQuery2" true)))
  ;[1 1 1] Get the object the cursor is hovering over.
  (bind _asmall_agent_character (cast `MallAgentCharacter` _hitactor)
    (:`then`
      (set `self.HoverActor` _asmall_agent_character))
    (:`CastFailed`
      (bind _asmall_interactable_master (cast `/Game/Blueprints/Mall/MallInteractable_Master` _hitactor)
        (:`then`
          (set `self.HoverActor` _asmall_interactable_master))
        (:`CastFailed`
          (bind _asplacement_zone (cast `/Game/Blueprints/Mall/PlacementZone` _hitactor)
            (:`then`
              (set `self.HoverActor` _asplacement_zone))
            (:`CastFailed`
              (set `self.HoverActor` null))))))))

(event `Key|LeftMouseButton`
  (params (Key :type "Key Structure"))
  ;[1 1 1] Select the object being hovered over.
  (:`Pressed`
    (`WidgetLayoutLibrary.RemoveAllWidgets`)
    (bind _output_get (set `self.HitActor` (`self.HoverActor`)))
    (cast `/Game/Blueprints/Agent/MallAgentCPP` _output_get
      (:`then`
        (bind _returnvalue (`|CreateWidget` "/Game/Blueprints/UI/AI_Debug_Tool.AI_Debug_Tool_C"))
        (`UserWidget.AddToViewport` _returnvalue 0))
      (:`CastFailed`
        (cast `/Game/Blueprints/Mall/MallInteractable_Master` _output_get
          (:`then`
            (bind _returnvalue_2 (`|CreateWidget` "/Game/Blueprints/UI/Interactable_Debug_Tool.Interactable_Debug_Tool_C"))
            (`UserWidget.AddToViewport` _returnvalue_2 0))
          (:`CastFailed`
            (cast `/Game/Blueprints/Mall/PlacementZone` _output_get)
            (bind _returnvalue_3 (`|CreateWidget` "/Game/Blueprints/UI/BuildingMenu.BuildingMenu_C"))
            (`UserWidget.AddToViewport` _returnvalue_3 0)))))))

(fn `MoveSpeedCalc`
  (returns (moveSensitivity :type "Float (double-precision)"))
  (return (`KismetMathLibrary.FClamp` (/ (`SpringArmComponent.TargetArmLength` (`/Game/Blueprints/Player/MallPlayerPawn.SpringArm` (`self.CameraPawn`))) 100.0) 5.0 20.0)))

(fn `UserConstructionScript`)